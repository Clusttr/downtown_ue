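; BP_BuildingProxy is an interactable building stand-in that pulses its construction floor indicator while selected.
; On BeginPlay it creates a dynamic material instance from GreenMat's parent and applies it to the indicator.
; Interact and StopInteract toggle IsSelected and start or stop the animation.
; A Timeline lerps SurfaceColor between Green and white, ping-ponging through OnColorLoop until deselection resets it to white.
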(event `self.ReceiveBeginPlay`
  ;[0 0 0] Make Dynamic Material
  (bind _returnvalue (`KismetMaterialLibrary.CreateDynamicMaterialInstance` (`MaterialInstance.Parent` (`self.GreenMat`))))
  (bind _output_get (set `self.Mat` _returnvalue))
  (`PrimitiveComponent.SetMaterial` (`self.ContrctionFloorIndicator`) 0 _output_get))

(event `/Game/Dynamic/Blueprints/Interactable/BI_Interactable.StopInteract`
  ;[0 0 0] Interaction
  (if (`self.IsSelected`)
    (`self.SetSelected` false)
    (`self.AnimateSelection` false)))

(event `AnimateSelection`
  (params (Value :type Boolean))
  ;[0 0 0] Floor Animation
  (if Value
    (set `self.CanLoopMat` true)
    (set `self.ColorLoopStart` true :!label _label)
    (bind (_direction _value) (`Timeline|Timeline` :!via `PlayFromStart` :!label _label_2)
      (:`Update`
        (`MaterialInstanceDynamic.SetVectorParameterValue` (`self.Mat`) "SurfaceColor" (`KismetMathLibrary.LinearColorLerp` (`self.Green`) (make `LinearColor` 1.0 1.0 1.0 1.0) _value)))
      (:`Finished`
        (`self.OnColorLoop`)))
    (else
      (set `self.CanLoopMat` false)
      (`|ExecutionSequence`
        (:`then_0`
          (goto _label_2 :!via `Stop`))
        (:`then_1`
          (`MaterialInstanceDynamic.SetVectorParameterValue` (`self.Mat`) "SurfaceColor" (struct :`R` 1.0 :`G` 1.0 :`B` 1.0 :`A` 1.0)))))))

(event `/Game/Dynamic/Blueprints/Interactable/BI_Interactable.Interact`
  ;[0 0 0] Interaction
  (if (not (`self.IsSelected`))
    (`self.SetSelected` true)
    (`self.AnimateSelection` true)))

(event `OnColorLoop`
  ;[0 0 0] Floor Animation
  (if (`self.CanLoopMat`)
    (if (`self.ColorLoopStart`)
      (set `self.ColorLoopStart` false)
      (goto _label_2 :!via `ReverseFromEnd`)
      (else
        (set `self.ColorLoopStart` true)
        (goto _label)))))

(fn `SetSelected`
  (params (Selected :type Boolean))
  (set `self.IsSelected` Selected))

(fn `UserConstructionScript`)