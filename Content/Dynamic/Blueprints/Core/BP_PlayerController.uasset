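; Player controller that detects whether the player is using gamepad, keyboard and mouse, or touch, and shows the mouse cursor.
; BeginPlay adds the IMC_Detection mapping context to supply the detection input actions.
; Gamepad key presses, non-zero IA_Move values and IA_TouchDetect each set InputType, calling KeySwitch only when the type changes.
; The IA_KeyDetect handler is empty, and a most-recent-hardware-device check is left unused.
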(event `self.ReceiveBeginPlay`
  (`EnhancedInputSubsystemInterface.AddMappingContext` (pcsubsystem `EnhancedInputLocalPlayerSubsystem` self) "/Game/Dynamic/Input/IMC_Detection.IMC_Detection" 0 (struct))
  (set `self.bShowMouseCursor` true))

(event `EnhancedInput|/Game/Dynamic/Input/Actions/IA_KeyDetect`
  (params (ActionValue :type Boolean) (ElapsedSeconds :type "Float (double-precision)") (TriggeredSeconds :type "Float (double-precision)") (InputAction :type "InputAction Object Reference" :default "/Game/Dynamic/Input/Actions/IA_KeyDetect.IA_KeyDetect")))

(event `Key|AnyKey`
  (params (Key :type "Key Structure"))
  (:`Pressed`
    (if (`KismetInputLibrary.Key_IsGamepadKey` Key)
      (switch `/Game/Dynamic/Input/E_InputType` (`self.InputType`)
        (:`NewEnumerator0`
          _)
        (:`NewEnumerator1`
          _)
        (:`NewEnumerator3`
          _))
      (set `self.InputType` "NewEnumerator2")
      (`self.KeySwitch` (`self.InputType`) :!label _label))))

(event `EnhancedInput|/Game/Dynamic/Input/Actions/IA_Move`
  (params (ActionValue :type "Vector2D Structure") (ElapsedSeconds :type "Float (double-precision)") (TriggeredSeconds :type "Float (double-precision)") (InputAction :type "InputAction Object Reference" :default "/Game/Dynamic/Input/Actions/IA_Move.IA_Move"))
  (:`Triggered`
    (if (!= (`KismetMathLibrary.VSize2D` ActionValue) 0.0)
      (switch `/Game/Dynamic/Input/E_InputType` (`self.InputType`)
        (:`NewEnumerator0`
          _)
        (:`NewEnumerator2`
          _)
        (:`NewEnumerator3`
          _))
      (set `self.InputType` "NewEnumerator1")
      (goto _label))))

(event `EnhancedInput|/Game/Dynamic/Input/Actions/IA_TouchDetect`
  (params (ActionValue :type Boolean) (ElapsedSeconds :type "Float (double-precision)") (TriggeredSeconds :type "Float (double-precision)") (InputAction :type "InputAction Object Reference" :default "/Game/Dynamic/Input/Actions/IA_TouchDetect.IA_TouchDetect"))
  (:`Started`
    (switch `/Game/Dynamic/Input/E_InputType` (`self.InputType`)
      (:`NewEnumerator0`
        _)
      (:`NewEnumerator1`
        _)
      (:`NewEnumerator2`
        _))
    (set `self.InputType` "NewEnumerator3")
    (goto _label)))

(fn `UserConstructionScript`)