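; BP_MeshOverSpline is an actor that tiles a static mesh along a spline as deformed segments.
; On construction, GenerateMesh adds collision-enabled spline mesh components at intervals of the mesh's X bounds length, clamping tangents to that length and omitting any partial final segment.
; An unwired Connect function would snap the last spline point's location and tangent to a tagged BP_CrossRoad spline's first point, with debug prints.
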(fn `Connect`
  (bind _spline (`self.Spline`))
  (bind _spline_2 (`self.Spline`))
  (bind (_actor _index _connect) (break `/Game/Dynamic/Structs/ST_SplineNodeData` (`self.Start Node`)))
  (bind _returnvalue (- (`SplineComponent.GetNumberOfSplinePoints` _spline) 1))
  (if (!= _actor null)
    (bind _asbp_cross_road (cast `/Game/Dynamic/Blueprints/Env/BP_CrossRoad` _actor))
    (bind _spline_3 (`/Game/Dynamic/Blueprints/Env/BP_CrossRoad.GetSplineWithTag` _asbp_cross_road (`KismetStringLibrary.Conv_StringToName` (`KismetStringLibrary.Conv_IntToString` _index))))
    (if _connect
      (bind (_location _tangent) (`SplineComponent.GetLocationAndTangentAtSplinePoint` _spline_3 0 "World"))
      (`KismetSystemLibrary.PrintString` (`KismetStringLibrary.Conv_VectorToString` _location))
      (`KismetSystemLibrary.PrintString` "Hello")
      (`SplineComponent.SetLocationAtSplinePoint` _spline _returnvalue _location "World" true)
      (`SplineComponent.SetTangentAtSplinePoint` _spline _returnvalue _tangent "World" true)
      (set `SplineComponent.bInputSplinePointsToConstructionScript` true _spline_2)
      (set `SplineComponent.bInputSplinePointsToConstructionScript` false _spline_2))))

(fn `GenerateMesh`
  (bind _spline (`self.Spline`))
  (bind _spline_2 (`self.Spline`))
  (bind (_returnvalue_min _returnvalue_max) (break `Box` (`StaticMesh.GetBoundingBox` (`self.Mesh`))))
  (bind _returnvalue_x (`KismetMathLibrary.BreakVector` (+ (`KismetMathLibrary.Vector_GetAbs` _returnvalue_min) (`KismetMathLibrary.Vector_GetAbs` _returnvalue_max))))
  (bind _output_get (set `self.XLength` _returnvalue_x))
  (for _index (range (`KismetMathLibrary.FTrunc` (/ (`SplineComponent.GetSplineLength` (`self.Spline`)) _output_get)))
    (bind _returnvalue (`AddComponent|NODE_AddSplineMeshComponent-0`))
    (`PrimitiveComponent.SetCollisionEnabled` _returnvalue "QueryAndPhysics")
    (`SplineMeshComponent.SetForwardAxis` _returnvalue "X" true)
    (`StaticMeshComponent.SetStaticMesh` _returnvalue (`self.Mesh`))
    (bind _returnvalue_2 (* _index (`self.XLength`)))
    (bind _returnvalue_3 (* (+ _index 1) (`self.XLength`)))
    (`SplineMeshComponent.SetStartAndEnd` _returnvalue (`SplineComponent.GetLocationAtDistanceAlongSpline` _spline_2 _returnvalue_2 "Local") (`KismetMathLibrary.ClampVectorSize` (`SplineComponent.GetTangentAtDistanceAlongSpline` _spline_2 _returnvalue_2 "Local") 0.0 (`self.XLength`)) (`SplineComponent.GetLocationAtDistanceAlongSpline` _spline _returnvalue_3 "Local") (`KismetMathLibrary.ClampVectorSize` (`SplineComponent.GetTangentAtDistanceAlongSpline` _spline _returnvalue_3 "Local") 0.0 (`self.XLength`)) true)))

(fn `UserConstructionScript`
  (`self.GenerateMesh`))